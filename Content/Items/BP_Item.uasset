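; BP_Item is an item actor that shows an on-screen interaction prompt while a player is within interaction range.
; On range enter it builds a BP_Interactive_Widget in a runtime-added, collision-free, screen-space widget component, then destroys that component on exit.
; GetInteractionText and InteractionTextAttach supply the prompt's text and attach point, defaulting to "Interact" and the root component.
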(event EventOnInteractionRangeEnter
  (params (Player :type Character%20Object%20Reference))
  (Variables|Private|GetInteractionWidgetComponent
    (:then)
    (:else
      (bind _returnvalue (Game|ConstructObjectfromClass "/Game/InteractiveInterface/BP_Interactive_Widget.BP_Interactive_Widget_C" (.AsPlayer%20Controller (Utilities|Casting|CastToPlayerController (Pawn|GetController Player))) (Private|GetInteractionText)))
      (bind _returnvalue_2 (AddComponent|AddWidgetComponent false))
      (bind _output_get (Variables|Private|SetInteractionWidgetComponent _returnvalue_2))
      (UserInterface|SetWidget _output_get _returnvalue)
      (Class|WidgetComponent|SetWidgetSpace _output_get "Screen")
      (Class|WidgetComponent|SetDrawatDesiredSize _output_get true)
      (Collision|SetCollisionEnabled _output_get "NoCollision")
      (Transformation|AttachComponentToComponent _output_get (Private|InteractionTextAttach) "None" "SnapToTarget" "SnapToTarget" "SnapToTarget" true))))

(event EventOnInteractionRangeExit
  (bind _interactionwidgetcomponent (Variables|Private|GetInteractionWidgetComponent)
    (:then
      (Components|DestroyComponent _interactionwidgetcomponent))
    (:else)))

(fn ConstructionScript)

(fn GetInteractionText
  (return "Interact"))

(fn InteractionTextAttach
  (return (Variables|Default|GetDefaultSceneRoot)))
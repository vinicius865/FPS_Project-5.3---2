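; Pickup gun that starts Dropped with physics on and hands itself to the interacting player, switching to Equipped with collision and physics off.
; SetGunState drives both pickup and Drop.
; Fire runs a debug-drawn line trace along the muzzle socket's up vector and adds a particle effect; it applies no damage, and the BP_Bullet spawn is unconnected.
; CurrentAmmo and Reload edit ammo counts stored on player 0's Ue4ASP_Character.
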(event Collision|EventActorBeginOverlap
  (params (OtherActor :type Actor%20Object%20Reference)))

(event EventTick
  (params (DeltaSeconds :type Float%20%28single-precision%29)))

(event EventOnInteractedPlayer
  (params (Player :type Ue%204ASP%20Character%20Object%20Reference))
  (Default|PickUpWeapon Player self)
  (Private|SetGunState "NewEnumerator1"))

(event EventBeginPlay
  (Private|SetGunState "NewEnumerator0"))

(fn ConstructionScript
  (|CallParentFunction))

(fn GetInteractionText
  (return "Pick Up"))

(fn InteractionTextAttach
  (return (Variables|Components|GetRfiel)))

(fn SetGunState
  (params (New%20Gun%20State :type EnumGunState%20Enum :default "NewEnumerator0"))
  (bind _rfiel (Variables|Components|GetRfiel))
  (bind _rfiel_2 (Variables|Components|GetRfiel))
  (bind _output_get (Variables|Private|SetGun%20State New%20Gun%20State))
  (switch Utilities|FlowControl|Switch|SwitchonEnumGunState _output_get
    (:NewEnumerator0
      (Collision|SetCollisionProfileName (Variables|Components|GetSphere) "OverlapAllDynamic" true :!class /Script/Engine.PrimitiveComponent)
      (Physics|SetSimulatePhysics _rfiel_2 true)
      (Collision|SetCollisionProfileName _rfiel_2 "DropWeapon" true :!class /Script/Engine.PrimitiveComponent))
    (:NewEnumerator1
      (Collision|SetCollisionProfileName (Variables|Components|GetSphere) "NoCollision" true :!class /Script/Engine.PrimitiveComponent)
      (Physics|SetSimulatePhysics _rfiel false)
      (Collision|SetCollisionProfileName _rfiel "NoCollision" true :!class /Script/Engine.PrimitiveComponent)
      (Transformation|ResetRelativeTransform _rfiel))))

(fn Drop
  (Private|SetGunState "NewEnumerator0"))

(fn Fire
  (params (PlayerCamera :type Camera%20Component%20Object%20Reference))
  (bind _rfiel (Variables|Components|GetRfiel))
  (bind _returnvalue (Transformation|GetSocketTransform _rfiel "b_gun_muzzleflash" "RTS_World"))
  (bind _returnvalue_2 (Transformation|GetSocketLocation _rfiel "b_gun_muzzleflash"))
  (bind (_outhit _returnvalue_3) (Collision|LineTraceByChannel (.location _returnvalue) (+ (.location _returnvalue) (* (Math|Vector|GetUpVector (.rotation _returnvalue)) 3e+04)) "TraceTypeQuery1" false 0 "ForDuration"))
  (AddComponent|AddParticleSystemComponent self true (Math|Transform|MakeTransform _returnvalue_2 (Math|Rotator|MakeRotator (.roll (Math|Rotator|FindLookatRotation _returnvalue_2 (Math|Vector|SelectVector (.ImpactNormal (Collision|BreakHitResult _outhit)) (.TraceEnd (Collision|BreakHitResult _outhit)) _returnvalue_3))) (+ (.pitch (Math|Rotator|FindLookatRotation _returnvalue_2 (Math|Vector|SelectVector (.ImpactNormal (Collision|BreakHitResult _outhit)) (.TraceEnd (Collision|BreakHitResult _outhit)) _returnvalue_3))) 0.0) (.yaw (Math|Rotator|FindLookatRotation _returnvalue_2 (Math|Vector|SelectVector (.ImpactNormal (Collision|BreakHitResult _outhit)) (.TraceEnd (Collision|BreakHitResult _outhit)) _returnvalue_3))))))
  (return))

(fn CurrentAmmo
  ;[1 1 1] Subtract current ammo minus one
  (bind _asue_4asp_character (Utilities|Casting|CastToUe4ASP_Character (Game|GetPlayerCharacter 0)))
  (if (> (Variables|/Game/ThirdPersonBP/Blueprints/Ue4ASP_Character.Ue4ASP_Character_C|GetcurrentAmmo _asue_4asp_character) 0)
    ;[0.4169 0.4338 0.6302] set New value for current Ammo
    (Variables|/Game/ThirdPersonBP/Blueprints/Ue4ASP_Character.Ue4ASP_Character_C|SetcurrentAmmo _asue_4asp_character (- (Variables|/Game/ThirdPersonBP/Blueprints/Ue4ASP_Character.Ue4ASP_Character_C|GetcurrentAmmo _asue_4asp_character) 1))
    (else
      ;[0.4586 0.6198 0.4552] If breanch is false, ammo is empty
      (Variables|/Game/ThirdPersonBP/Blueprints/Ue4ASP_Character.Ue4ASP_Character_C|SetammoIsEmpty _asue_4asp_character true))))

(fn Reload
  (bind _asue_4asp_character (Utilities|Casting|CastToUe4ASP_Character (Game|GetPlayerCharacter 0)))
  (if (< (Variables|/Game/ThirdPersonBP/Blueprints/Ue4ASP_Character.Ue4ASP_Character_C|GetcurrentAmmo _asue_4asp_character) (Variables|/Game/ThirdPersonBP/Blueprints/Ue4ASP_Character.Ue4ASP_Character_C|GetclipSize _asue_4asp_character))
    (if (> (Variables|/Game/ThirdPersonBP/Blueprints/Ue4ASP_Character.Ue4ASP_Character_C|GetmaxAmmo _asue_4asp_character) (- (Variables|/Game/ThirdPersonBP/Blueprints/Ue4ASP_Character.Ue4ASP_Character_C|GetclipSize _asue_4asp_character) (Variables|/Game/ThirdPersonBP/Blueprints/Ue4ASP_Character.Ue4ASP_Character_C|GetcurrentAmmo _asue_4asp_character)))
      (Variables|Default|SetammoDifference (- (Variables|/Game/ThirdPersonBP/Blueprints/Ue4ASP_Character.Ue4ASP_Character_C|GetclipSize _asue_4asp_character) (Variables|/Game/ThirdPersonBP/Blueprints/Ue4ASP_Character.Ue4ASP_Character_C|GetcurrentAmmo _asue_4asp_character)))
      (Variables|/Game/ThirdPersonBP/Blueprints/Ue4ASP_Character.Ue4ASP_Character_C|SetcurrentAmmo _asue_4asp_character (+ (Variables|/Game/ThirdPersonBP/Blueprints/Ue4ASP_Character.Ue4ASP_Character_C|GetcurrentAmmo _asue_4asp_character) (Variables|Default|GetammoDifference)))
      (Variables|/Game/ThirdPersonBP/Blueprints/Ue4ASP_Character.Ue4ASP_Character_C|SetmaxAmmo _asue_4asp_character (- (Variables|/Game/ThirdPersonBP/Blueprints/Ue4ASP_Character.Ue4ASP_Character_C|GetmaxAmmo _asue_4asp_character) (Variables|Default|GetammoDifference)))
      (bind _output_get (Variables|/Game/ThirdPersonBP/Blueprints/Ue4ASP_Character.Ue4ASP_Character_C|SetisReloading _asue_4asp_character true))
      (return _output_get (stale _output_get_2))
      (else
        (Variables|Default|SetammoDifference (- (Variables|/Game/ThirdPersonBP/Blueprints/Ue4ASP_Character.Ue4ASP_Character_C|GetclipSize _asue_4asp_character) (Variables|/Game/ThirdPersonBP/Blueprints/Ue4ASP_Character.Ue4ASP_Character_C|GetcurrentAmmo _asue_4asp_character)))
        (Variables|/Game/ThirdPersonBP/Blueprints/Ue4ASP_Character.Ue4ASP_Character_C|SetcurrentAmmo _asue_4asp_character (+ (Variables|/Game/ThirdPersonBP/Blueprints/Ue4ASP_Character.Ue4ASP_Character_C|GetcurrentAmmo _asue_4asp_character) (Variables|/Game/ThirdPersonBP/Blueprints/Ue4ASP_Character.Ue4ASP_Character_C|GetmaxAmmo _asue_4asp_character)))
        (Variables|/Game/ThirdPersonBP/Blueprints/Ue4ASP_Character.Ue4ASP_Character_C|SetmaxAmmo _asue_4asp_character 0)
        (bind _output_get_2 (Variables|/Game/ThirdPersonBP/Blueprints/Ue4ASP_Character.Ue4ASP_Character_C|SetisReloading _asue_4asp_character true))))
    (else
      (Development|PrintString "Full ammo"))))